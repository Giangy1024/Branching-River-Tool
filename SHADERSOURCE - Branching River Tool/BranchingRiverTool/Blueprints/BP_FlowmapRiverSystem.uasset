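; Spline-based river actor for building branching rivers that can attach to points on other rivers.
; Construction attaches it to any parent river, builds a tagged spline mesh per segment with main and LOD materials, and adds optional index and flow-arrow visualizers.
; Split points halve and sideways-offset segment starts, while attached rivers take location, tangent and starting width from the parent point.
; UpdateRiver syncs the split array, refreshes meshes and propagates recursively to attached rivers.
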(event Custom|UpdateRiver
  (bind _riversplinecomponent (Variables|Default|GetRiverSplineComponent))
  (CallFunction|RefreshRiverSplits)
  (bind _index (Utilities|LoopThroughSplines true _riversplinecomponent)
    (:Loop
      (CallFunction|UpdateRiverMeshesScaleLocationTangent _riversplinecomponent _index)
      (CallFunction|UpdateRiverSplines))
    (:Completed
      (for _array_element (Actor|GetAttachedActors true)
        (bind _asbp_flowmap_river_system (Utilities|Casting|CastToBP_FlowmapRiverSystem _array_element))
        (CallFunction|UpdateRiver _asbp_flowmap_river_system)))))

(event EventBeginPlay)

(event Collision|EventActorBeginOverlap
  (params (OtherActor :type Actor%20Object%20Reference)))

(event EventTick
  (params (DeltaSeconds :type Float%20%28single-precision%29)))

(fn ConstructionScript
  ;[1 1 1] Construct Functions
  (CallFunction|SetupAttachment)
  (CallFunction|SetupRiverMeshes)
  (CallFunction|SetupSplineVisualizers))

(fn SetupRiverMeshes
  (bind _riversplinecomponent (Variables|Default|GetRiverSplineComponent))
  ;[1 1 1] Clear Spline Mesh Component Array
  (Utilities|Array|Clear (Variables|Default|GetRiverSplineMeshComponents))
  ;[1 1 1] Loop Through Spline Points
  (bind _index (Utilities|LoopThroughSplines true _riversplinecomponent)
    (:Loop
      ;[1 1 1] Add Spline Mesh Component, Add to Component Array
      (bind _returnvalue (AddComponent|AddSplineMeshComponent false))
      (Variables|/Script/Engine.ActorComponent|SetComponentTags _returnvalue (Utilities|Array|MakeArray (Variables|FluidInteractionTool|GetFluidSurfaceTag)))
      ;[1 1 1] Update River Meshes Scale Location Tangent
      (Utilities|Array|Add (Variables|Default|GetRiverSplineMeshComponents) _returnvalue)
      (CallFunction|UpdateRiverMeshesScaleLocationTangent _riversplinecomponent _index)
      ;[1 1 1] Setup Material and LOD Material
      (Rendering|Material|SetMaterialbyName _returnvalue "Main" (Variables|Default|GetRiverMaterial))
      (Rendering|Material|SetMaterialbyName _returnvalue "Cheap" (Variables|Default|GetRiverMaterial_LOD)))))

(fn SetupSplineVisualizers
  (bind _riversplinecomponent (Variables|Default|GetRiverSplineComponent))
  ;[1 1 1] Check if we want to show Visualizers
  (if (Variables|Visualizers|GetShowSplineVisualizers)
    ;[1 1 1] Loop Through Splines
    (bind _index (Utilities|LoopThroughSplines false _riversplinecomponent)
      (:Loop
        (Utilities|FlowControl|Sequence
          (:then_0
            ;[1 1 1] Setup Text Render for spline point index
            (if (Variables|Visualizers|GetShowSplineNumber)
              (bind _returnvalue (AddComponent|AddTextRenderComponent false (Math|Transform|MakeTransform (Math|Vector|MakeVector (.x (Spline|GetLocationatSplinePoint _riversplinecomponent _index "Local")) (.y (Spline|GetLocationatSplinePoint _riversplinecomponent _index "Local")) (+ (.z (Spline|GetLocationatSplinePoint _riversplinecomponent _index "Local")) 64.0)) "0, 0, 0" (Math|Conversions|ToVector(Float) (Variables|Visualizers|GetSplineNumberSize)))))
              (Rendering|Components|TextRender|SetText _returnvalue (Utilities|Text|ToText(Integer) _index))
              (Rendering|Components|TextRender|SetTextRenderColor _returnvalue (Variables|Visualizers|GetSplineNumberColor))))
          (:then_1
            ;[1 1 1] Setup Direction Arrow for water flow direction
            (if (Variables|Visualizers|GetShowSplineDirection)
              (bind _returnvalue_2 (AddComponent|AddArrowComponent false (Math|Transform|MakeTransform (Math|Vector|MakeVector (.x (Spline|GetLocationatSplinePoint _riversplinecomponent _index "Local")) (.y (Spline|GetLocationatSplinePoint _riversplinecomponent _index "Local")) (+ (.z (Spline|GetLocationatSplinePoint _riversplinecomponent _index "Local")) 64.0)) (Math|Rotator|MakeRotator (.roll (Math|Conversions|RotationFromXVector (Class|SplineComponent|GetRightVectoratSplinePoint (Variables|Default|GetRiverSplineComponent) _index "Local"))) (.pitch (Math|Conversions|RotationFromXVector (Class|SplineComponent|GetRightVectoratSplinePoint (Variables|Default|GetRiverSplineComponent) _index "Local"))) (+ (.yaw (Math|Conversions|RotationFromXVector (Class|SplineComponent|GetRightVectoratSplinePoint (Variables|Default|GetRiverSplineComponent) _index "Local"))) -9e+01)) (Math|Conversions|ToVector(Float) (Variables|Visualizers|GetSplineDirectionSize)))))
              (Variables|/Script/Engine.ArrowComponent|SetArrowColor _returnvalue_2 (Variables|Visualizers|GetSplineDirectionColor)))))))))

(fn RefreshRiverSplits
  (bind _riversplits (Variables|Default|GetRiverSplits))
  (bind _riversplinecomponent (Variables|Default|GetRiverSplineComponent))
  (bind _riversplits_2 (Variables|Default|GetRiverSplits))
  ;[1 1 1] Loop through spiles and collect index's
  (bind _index (Utilities|LoopThroughSplines false _riversplinecomponent)
    (:Loop
      (if (not (Utilities|Array|IsValidIndex _riversplits _index))
        (Utilities|Array|Add _riversplits "NewEnumerator0")))
    (:Completed
      (for (_ _array_index) _riversplits_2
        (if (> _array_index (- (Spline|GetNumberOfSplinePoints _riversplinecomponent) 1))
          (Utilities|Array|RemoveIndex _riversplits_2 _array_index))))))

(fn SetupAttachment
  (bind _riverattachment (Variables|Default|GetRiverAttachment))
  (bind _rivertoattachto (Utilities|Struct|BreakStruct_AttachRiver _riverattachment))
  ;[1 1 1] Setup River Attachment and then update River Splines
  (Utilities|IsValid _rivertoattachto
    (:Is%20Valid
      (Transformation|AttachActorToActor _rivertoattachto "None" "SnapToTarget" "KeepWorld" "KeepWorld" true)
      (CallFunction|UpdateRiverSplines))))

(fn UpdateRiverMeshesScaleLocationTangent
  (params (RiverSplineComponent :type Spline%20Component%20Object%20Reference%20%28by%20ref%29) (Index :type Integer))
  (bind _returnvalue (== Index 0))
  (bind (_location _tangent) (Spline|GetLocationandTangentatSplinePoint RiverSplineComponent Index "Local"))
  (bind _returnvalue_2 (+ Index 1))
  (bind _returnvalue_3 (Utilities|Enum|LiteralenumEnum_RiverBranching "NewEnumerator2"))
  (bind _returnvalue_4 (Utilities|Enum|LiteralenumEnum_RiverBranching "NewEnumerator1"))
  (bind _overallscale (Variables|Default|GetOverallScale))
  (bind _riversplits (Variables|Default|GetRiverSplits))
  (bind _riverattachment (Variables|Default|GetRiverAttachment))
  (bind _riversplinemeshcomponents (Variables|Default|GetRiverSplineMeshComponents))
  (bind (_rivertoattachto _attachmentindex) (Utilities|Struct|BreakStruct_AttachRiver _riverattachment))
  (bind (_location_2 _tangent_2) (Spline|GetLocationandTangentatSplinePoint RiverSplineComponent _returnvalue_2 "Local"))
  (bind _output (Utilities|Array|Get(acopy) _riversplits Index))
  (bind _output_2 (Utilities|Array|Get(acopy) _riversplinemeshcomponents Index))
  (bind _returnvalue_5 (Utilities|IsValid _rivertoattachto))
  (bind _returnvalue_6 (Utilities|Enum|Equal(Enum) _output _returnvalue_4))
  (bind _returnvalue_7 (Utilities|Enum|Equal(Enum) _output _returnvalue_3))
  (bind _returnvalue_8 (and _returnvalue_5 _returnvalue))
  (bind _returnvalue_9 (select _returnvalue_8 (Variables|BP_FlowmapRiverSystem_C|GetRiverSplineComponent _rivertoattachto) RiverSplineComponent))
  (bind _returnvalue_10 (select _returnvalue_8 _attachmentindex Index))
  (bind _returnvalue_11 (Spline|GetScaleatSplinePoint _returnvalue_9 _returnvalue_10))
  (bind _returnvalue_12 (* (.y _returnvalue_11) _overallscale))
  (Utilities|FlowControl|Sequence
    (:then_0
      ;[1 1 1] Set Start End Location and Tangent
      (SplineMesh|SetStartandEnd _output_2 (select (or _returnvalue_6 _returnvalue_7) (+ (/ (* (Class|SplineComponent|GetRightVectoratSplinePoint RiverSplineComponent Index "Local") (* (select _returnvalue_7 2.5e+02 -2.5e+02) _returnvalue_12)) 2.0) _location) _location) _tangent _location_2 _tangent_2 true :!class /Script/Engine.SplineMeshComponent))
    (:then_1
      ;[1 1 1] Set Spline Mesh Scale Depending on the River Split
      (SplineMesh|SetStartScale _output_2 (Math|Vector2D|MakeVector2D (select (or _returnvalue_6 _returnvalue_7) (/ _returnvalue_12 2.0) _returnvalue_12) 1.0) true :!class /Script/Engine.SplineMeshComponent))
    (:then_2
      (SplineMesh|SetEndScale _output_2 (Math|Vector2D|MakeVector2D (* (.y (Spline|GetScaleatSplinePoint RiverSplineComponent (+ Index 1))) _overallscale) 1.0) true :!class /Script/Engine.SplineMeshComponent))))

(fn UpdateRiverSplines
  (bind _riverattachment (Variables|Default|GetRiverAttachment))
  (bind _riversplinecomponent (Variables|Default|GetRiverSplineComponent))
  (bind _riversplinecomponent_2 (Variables|BP_FlowmapRiverSystem_C|GetRiverSplineComponent (.rivertoattachto _riverattachment)))
  (bind (_location _tangent) (Spline|GetLocationandTangentatSplinePoint _riversplinecomponent_2 (.attachmentindex _riverattachment) "World"))
  ;[1 1 1] Update Location and Tangent for Attachment
  (Utilities|IsValid (.rivertoattachto _riverattachment)
    (:Is%20Valid
      (Transformation|SetActorLocation _location false true)
      (Spline|SetLocationatSplinePoint _riversplinecomponent 0 _location "World" true)
      (Spline|SetTangentatSplinePoint _riversplinecomponent 0 _tangent "World" true))))